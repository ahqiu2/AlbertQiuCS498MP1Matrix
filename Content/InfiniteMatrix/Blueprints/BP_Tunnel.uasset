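; BP_Tunnel is a tunnel segment with a spinning holed wall; RandomizeWall picks one of four hole meshes and a random roll.
; Player overlap with TriggerZone has TunnelSpawner spawn the next tunnel, an enemy and occasionally health, destroys this segment, and scores unless TookDamage is set.
; Wall hits damage the player, briefly disable the player's collision, and set TookDamage for the same short delay.
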(event OnComponentHit(WallMesh)
  (params (HitComponent :type Primitive%20Component%20Object%20Reference) (OtherActor :type Actor%20Object%20Reference) (OtherComp :type Primitive%20Component%20Object%20Reference) (NormalImpulse :type Vector :default "0, 0, 0") (Hit :type Hit%20Result%20Structure%20%28by%20ref%29))
  (bind _asbp_player (Utilities|Casting|CastToBP_Player OtherActor))
  (Default|TakeDamage _asbp_player)
  (Utilities|FlowControl|Sequence
    (:then_0
      (bind _asbp_player_2 (Utilities|Casting|CastToBP_Player OtherActor))
      (Collision|SetActorEnableCollision _asbp_player_2 false)
      (Utilities|FlowControl|Delay 0.05)
      (bind _asbp_player_3 (Utilities|Casting|CastToBP_Player OtherActor))
      (Collision|SetActorEnableCollision _asbp_player_3 true))
    (:then_1
      (Variables|Default|SetTook%20Damage true)
      (Utilities|FlowControl|Delay 0.05)
      (Variables|Default|SetTook%20Damage false))))

(event OnComponentBeginOverlap(TriggerZone)
  (params (OverlappedComponent :type Primitive%20Component%20Object%20Reference) (OtherActor :type Actor%20Object%20Reference) (OtherComp :type Primitive%20Component%20Object%20Reference) (OtherBodyIndex :type Integer) (bFromSweep :type Boolean) (SweepResult :type Hit%20Result%20Structure%20%28by%20ref%29))
  (Utilities|Casting|CastToBP_Player OtherActor)
  (Utilities|FlowControl|Sequence
    (:then_0
      (Default|SpawnTunnelatSpawnPoint (Variables|Components|GetTunnelSpawner))
      (Actor|DestroyActor)
      (bind _asbp_player (Utilities|Casting|CastToBP_Player OtherActor))
      (if (not (Variables|Default|GetTook%20Damage))
        (Default|IncreaseScore _asbp_player)))
    (:then_1
      (Math|Integer|CompareInt (Math|Random|RandomInteger 5) 1
        (:<
          (Default|SpawnHealthatSpawn (Variables|Components|GetTunnelSpawner)))))
    (:then_2
      (Default|SpawnEnemyatSpawn (Variables|Components|GetTunnelSpawner)))))

(event EventBeginPlay)

(event EventTick
  (params (DeltaSeconds :type Float%20%28single-precision%29))
  (Transformation|AddLocalRotation (Variables|Components|GetWallMesh) (Math|Rotator|MakeRotator (* DeltaSeconds (Variables|Default|GetRotateSpeed)) 0.0 0.0) false false))

(fn ConstructionScript)

(fn RandomizeWall
  (Components|StaticMesh|SetStaticMesh (Variables|Components|GetWallMesh) (Utilities|Select :Index (Math|Random|RandomIntegerinRange 0 3) :Option%200 "/Game/InfiniteMatrix/Meshes/SM_Hole_01.SM_Hole_01" :Option%201 "/Game/InfiniteMatrix/Meshes/SM_Hole_02.SM_Hole_02" :Option%202 "/Game/InfiniteMatrix/Meshes/SM_Hole_03.SM_Hole_03" :Option%203 "/Game/InfiniteMatrix/Meshes/SM_Hole_04.SM_Hole_04"))
  (Transformation|AddLocalRotation (Variables|Components|GetWallMesh) (Math|Rotator|MakeRotator (Math|Random|RandomFloatinRange 0.0 3.6e+02) 0.0 0.0) false false))